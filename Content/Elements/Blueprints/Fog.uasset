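; Fog projectile actor that flies along its facing direction, shrinks and then fades out.
; On BeginPlay it rotates a velocity vector by its own rotation for the projectile movement, while a timeline gradually scales the actor down.
; When the timeline finishes, it toggles the particle effect off and waits so particles fade before destroying itself.
; Overlap and hit events are empty.
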(event `self.ReceiveBeginPlay`
  (set `MovementComponent.Velocity` (`KismetMathLibrary.GreaterGreater_VectorRotator` (`self.Velocity`) (`self.K2_GetActorRotation`)) (`self.ProjectileMovement1`)) ; Set the speed/direction of the projectile
  (bind (_direction _scale) (`Timeline|Timeline_0`) ; Timeline blends from 1 to 0.15
    (:`Update`
      (`self.SetActorRelativeScale3D` (* (`KismetMathLibrary.MakeVector` 1.0 1.0 1.0) _scale)) ; Gradually shrink the actor
    )
    (:`Finished`
      (`ActorComponent.ToggleActive` (`self.Effect`)) ; Turn off effect to give particles a chance to fade instead of disappearing suddenly when the actor is destroyed
      (`KismetSystemLibrary.Delay` 10.0)
      (`self.K2_DestroyActor`))))

(event `self.ReceiveActorBeginOverlap`
  (params (OtherActor :type "Actor Object Reference")))

(event `self.ReceiveHit`
  (params (MyComp :type "PrimitiveComponent Object Reference") (Other :type "Actor Object Reference") (OtherComp :type "PrimitiveComponent Object Reference") (bSelfMoved :type Boolean) (HitLocation :type "Vector Structure") (HitNormal :type "Vector Structure") (NormalImpulse :type "Vector Structure") (Hit :type "HitResult Structure (by ref)")))

(fn `UserConstructionScript`)