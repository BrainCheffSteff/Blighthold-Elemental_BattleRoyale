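; Air dart projectile, owned by a UWOT_BaseCharacter, that bursts on impact.
; On spawn it aligns velocity to its rotation, briefly ignores owner collision, then shrinks via timeline until destroyed.
; Hits on characters set the victim's hit direction and the owner's damage flag.
; Every owned hit triggers burst particles, radial force and sound, but only player 0's darts call the owner's ExplosionEvent for damage and voxel effects.
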(event `self.ReceiveBeginPlay`
  (bind _asuwot_base_character (cast `/Game/ThirdPersonCPP/Characters/UWOT_BaseCharacter` (`self.GetOwner`))
    (:`then`
      (set `MovementComponent.Velocity` (`KismetMathLibrary.GreaterGreater_VectorRotator` (`self.Velocity`) (`self.K2_GetActorRotation`)) (`self.ProjectileMovement1`)) ; Set the speed/direction of the projectile
      (`PrimitiveComponent.IgnoreActorWhenMoving` (`self.Collision`) _asuwot_base_character true)
      (bind _capsulecomponent (`Character.CapsuleComponent` _asuwot_base_character))
      (`PrimitiveComponent.IgnoreActorWhenMoving` _capsulecomponent self true)
      (`KismetSystemLibrary.Delay` 0.25)
      (`PrimitiveComponent.IgnoreActorWhenMoving` (`self.Collision`) _asuwot_base_character false)
      (`PrimitiveComponent.IgnoreActorWhenMoving` _capsulecomponent self false)
      (bind (_direction _scale) (`Timeline|LifeSpan`) ; Timeline blends from 1 to 0.15
        (:`Update`
          (`self.SetActorRelativeScale3D` (* (`KismetMathLibrary.MakeVector` 1.0 1.0 1.0) _scale)) ; Gradually shrink the actor
        )
        (:`Finished`
          (`ActorComponent.ToggleActive` (`self.Effect`)) ; Turn off effect to give particles a chance to fade instead of disappearing suddenly when the actor is destroyed
          (`KismetSystemLibrary.Delay` 0.1)
          (`self.K2_DestroyActor`))))
    (:`CastFailed`
      (`KismetSystemLibrary.PrintString` "FUCKITTY"))))

(event `self.ReceiveActorBeginOverlap`
  (params (OtherActor :type "Actor Object Reference")))

(event `self.ReceiveHit`
  (params (MyComp :type "PrimitiveComponent Object Reference") (Other :type "Actor Object Reference") (OtherComp :type "PrimitiveComponent Object Reference") (bSelfMoved :type Boolean) (HitLocation :type "Vector Structure") (HitNormal :type "Vector Structure") (NormalImpulse :type "Vector Structure") (Hit :type "HitResult Structure (by ref)"))
  (bind _returnvalue (`self.K2_GetActorLocation`))
  (bind _returnvalue_2 (`self.K2_GetActorRotation`))
  (bind _returnvalue_3 (`self.K2_GetActorLocation`))
  (bind _returnvalue_4 (`self.K2_GetActorRotation`))
  (bind _returnvalue_5 (`self.GetOwner`))
  (bind _asuwot_base_character (cast `/Game/ThirdPersonCPP/Characters/UWOT_BaseCharacter` Other)
    (:`then`
      (set `self.HitSomeone?` true)
      (set `/Game/ThirdPersonCPP/Characters/UWOT_BaseCharacter.GotHit?` (- (.yaw (`KismetMathLibrary.Conv_VectorToRotator` (`KismetMathLibrary.Normal` (* HitNormal (1.0 1.0 0.0))))) (.yaw (`KismetMathLibrary.Conv_VectorToRotator` (`KismetMathLibrary.Normal` (* (`SceneComponent.GetForwardVector` (`/Game/ThirdPersonCPP/Characters/UWOT_BaseCharacter.Camera` _asuwot_base_character)) (1.0 1.0 0.0)))))) _asuwot_base_character))
    (:`CastFailed`
      (set `self.HitSomeone?` false)))
  (set `self.Origin_` HitLocation)
  (bind _asuwot_base_character_2 (cast `/Game/ThirdPersonCPP/Characters/UWOT_BaseCharacter` (`self.GetOwner`)))
  (if (`self.HitSomeone?`)
    (set `/Game/ThirdPersonCPP/Characters/UWOT_BaseCharacter.DamagedSomeone_` 6.0 _asuwot_base_character_2))
  (if (== (`Pawn.PlayerState` _asuwot_base_character_2) (`Controller.PlayerState` (`GameplayStatics.GetPlayerController` 0)))
    (bind _asuwot_base_character_3 (cast `/Game/ThirdPersonCPP/Characters/UWOT_BaseCharacter` (`self.GetOwner`)))
    (`/Game/ThirdPersonCPP/Characters/UWOT_BaseCharacter.ExplosionEvent` _asuwot_base_character_3 (`self.DamageRadius`) (`self.Origin_`) _returnvalue_3 _returnvalue_4 (`self.ImpulseStrength`) (`self.Damage`) false (`self.GetInstigatorController` _returnvalue_5) _returnvalue_5 "/Script/Engine.DamageType" true 0.0)
    (`GameplayStatics.SpawnEmitterAtLocation` "/Game/Elements/Air/P_AirDart_Burst.P_AirDart_Burst" _returnvalue_3 _returnvalue_4)
    (`ActorComponent.Activate` (`self.RadialForce`) false)
    (`ActorComponent.ToggleActive` (`self.Effect`)) ; Turn off effect to give particles a chance to fade instead of disappearing suddenly when the actor is destroyed
    (`GameplayStatics.PlaySoundAtLocation` "/Game/StarterContent/Audio/Explosion_Cue.Explosion_Cue" (`self.K2_GetActorLocation`) (`self.K2_GetActorRotation`))
    (`KismetSystemLibrary.Delay` 0.05)
    (`self.K2_DestroyActor`)
    (else
      (`GameplayStatics.SpawnEmitterAtLocation` "/Game/Elements/Air/P_AirDart_Burst.P_AirDart_Burst" _returnvalue _returnvalue_2)
      (`ActorComponent.Activate` (`self.RadialForce`) false)
      (`GameplayStatics.PlaySoundAtLocation` "/Game/StarterContent/Audio/Fire_Sparks01_Cue.Fire_Sparks01_Cue" _returnvalue _returnvalue_2)
      (`KismetSystemLibrary.Delay` 0.05)
      (`self.K2_DestroyActor`))))

(fn `UserConstructionScript`)