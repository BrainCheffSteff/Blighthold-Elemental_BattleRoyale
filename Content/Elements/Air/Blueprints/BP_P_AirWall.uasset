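; BP_P_AirWall is an air-element wall with a shield component that shows a ripple-style effect where it is hit.
; On a ShieldBeta hit, it creates a dynamic material instance, sets its "Pos" parameter to the impact point and spawns a hit emitter facing along the impact normal.
; A timeline, replayed from the start on each hit, drives the material's "Radius" parameter to animate the effect.
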(event `self.ShieldBeta.OnComponentHit`
  (params (HitComponent :type "PrimitiveComponent Object Reference") (OtherActor :type "Actor Object Reference") (OtherComp :type "PrimitiveComponent Object Reference") (NormalImpulse :type "Vector Structure") (Hit :type "HitResult Structure (by ref)"))
  (bind _returnvalue (`PrimitiveComponent.CreateDynamicMaterialInstance` (`self.ShieldBeta`) 0 null))
  (`MaterialInstanceDynamic.SetVectorParameterValue` _returnvalue "Pos" (`KismetMathLibrary.Conv_VectorToLinearColor` Hit_ImpactPoint))
  (`GameplayStatics.SpawnEmitterAtLocation` "/Game/Elements/Air/ParticleEmitters/ShieldHitEffect.ShieldHitEffect" Hit_ImpactPoint (`KismetMathLibrary.Conv_VectorToRotator` Hit_ImpactNormal))
  (bind (_direction _newtrack_0) (`Timeline|HitEffectTimeline` :!via `PlayFromStart`)
    (:`Update`
      (`MaterialInstanceDynamic.SetScalarParameterValue` _returnvalue "Radius" (* _newtrack_0 75.0)))))

(fn `UserConstructionScript`
  (`parent.UserConstructionScript`))